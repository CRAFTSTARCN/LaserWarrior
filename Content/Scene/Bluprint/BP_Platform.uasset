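; BP_Platform is a pressure-button platform that runs an elevator while the player stands on it.
; On BeginPlay it hands its ProjectileMovement component to the Elevator.
; Sphere overlap events filtered to the player pawn fire ButtonPressed and ButtonReleased, which toggle the Elevator's RunStatus.
; The same events light or darken the CenterButton and Ring by setting their EmissiveScale material parameter.
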(event `self.ReceiveBeginPlay`
  (`ElevatorComponent.SetMovementComponent` (`self.Elevator`) (`self.ProjectileMovement`)))

(event `self.Sphere.OnComponentBeginOverlap`
  (params (OverlappedComponent :type "PrimitiveComponent Object Reference") (OtherActor :type "Actor Object Reference") (OtherComp :type "PrimitiveComponent Object Reference") (OtherBodyIndex :type Integer) (bFromSweep :type Boolean) (SweepResult :type "HitResult Structure (by ref)"))
  (if (== OtherActor (`GameplayStatics.GetPlayerPawn` 0))
    (`self.ButtonPressed`)))

(event `ButtonPressed`
  (bind _lightnessonpressed (`self.LightnessOnPressed`))
  (`MeshComponent.SetScalarParameterValueOnMaterials` (`self.Center Button`) "EmissiveScale" _lightnessonpressed)
  (`MeshComponent.SetScalarParameterValueOnMaterials` (`self.Ring`) "EmissiveScale" _lightnessonpressed)
  (set `ElevatorComponent.RunStatus` true (`self.Elevator`)))

(event `ButtonReleased`
  (`MeshComponent.SetScalarParameterValueOnMaterials` (`self.Center Button`) "EmissiveScale" 0.0)
  (`MeshComponent.SetScalarParameterValueOnMaterials` (`self.Ring`) "EmissiveScale" 0.0)
  (set `ElevatorComponent.RunStatus` false (`self.Elevator`)))

(event `self.Sphere.OnComponentEndOverlap`
  (params (OverlappedComponent :type "PrimitiveComponent Object Reference") (OtherActor :type "Actor Object Reference") (OtherComp :type "PrimitiveComponent Object Reference") (OtherBodyIndex :type Integer))
  (if (== OtherActor (`GameplayStatics.GetPlayerPawn` 0))
    (`self.ButtonReleased`)))

(fn `UserConstructionScript`)