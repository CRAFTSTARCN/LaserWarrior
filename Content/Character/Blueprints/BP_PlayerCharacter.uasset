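; Player character Blueprint for a sword-wielding samurai that supplies the animation and visual responses for combat and movement events.
; Events play montages for heavy attack, skill, dodges and hit reaction, falling stops the montage, and AttackAnimPlay picks one of four combo montages by index.
; The construction script attaches the weapon to the mesh socket and initializes HitBoxTrace with it.
; BeginPlay deactivates SwordTail, and ChangeHeartMaterial swaps an emissive material at low HP.
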(event `self.ReceiveBeginPlay`
  (`ActorComponent.Deactivate` (`self.Sword Tail`)))

(event `self.HeavyAttackAnimPlay`
  (`self.PlayAnimMontage` "/Game/Character/SamuraiAnimation/RootMotion/Anim_ARPGSamurai_Attack_Dodge_Montage.Anim_ARPGSamurai_Attack_Dodge_Montage"))

(event `self.ChangeHeartMaterial`
  (params (Percentage :type "Float (single-precision)"))
  (bind _mesh (`self.Mesh`))
  (if (< Percentage 0.5)
    (`PrimitiveComponent.SetMaterial` _mesh 1 "/Game/Character/Mannequin/Character/Materials/M_Emissive_Logo_Inst_Low_Hp.M_Emissive_Logo_Inst_Low_Hp")
    (else
      (`PrimitiveComponent.SetMaterial` _mesh 1 "/Game/Character/Mannequin/Character/Materials/M_Emissive_Logo_Inst.M_Emissive_Logo_Inst"))))

(event `self.PlayerFall`
  (`self.StopAnimMontage` null))

(event `self.PlayDodgeForward`
  (`self.PlayAnimMontage` "/Game/Character/SamuraiAnimation/RootMotion/Anim_ARPGSamurai_Evade_Forward_Montage.Anim_ARPGSamurai_Evade_Forward_Montage"))

(event `self.PlayDodgeBackward`
  (`self.PlayAnimMontage` "/Game/Character/SamuraiAnimation/RootMotion/Anim_ARPGSamurai_Dodge_Montage.Anim_ARPGSamurai_Dodge_Montage"))

(event `self.HittedAnimePlay`
  (`self.PlayAnimMontage` "/Game/Character/SamuraiAnimation/RootMotion/Anim_ARPGSamurai_Hit1_Montage.Anim_ARPGSamurai_Hit1_Montage"))

(event `self.SkillAnimePlay`
  (`self.PlayAnimMontage` "/Game/Character/SamuraiAnimation/RootMotion/Anim_ARPGSamurai_Attack_Heavy1_Montage.Anim_ARPGSamurai_Attack_Heavy1_Montage"))

(fn `AttackAnimPlay`
  (params (AttackComboNum :type Integer))
  (returns (ReturnValue :type "Float (double-precision)"))
  (bind _returnvalue (`self.PlayAnimMontage` (select `int` AttackComboNum :`0` "/Game/Character/SamuraiAnimation/RootMotion/Anim_ARPGSamurai_Attack_Combo1_Montage.Anim_ARPGSamurai_Attack_Combo1_Montage" :`1` "/Game/Character/SamuraiAnimation/RootMotion/Anim_ARPGSamurai_Attack_Combo2_Montage.Anim_ARPGSamurai_Attack_Combo2_Montage" :`2` "/Game/Character/SamuraiAnimation/RootMotion/Anim_ARPGSamurai_Attack_Combo3_Montage.Anim_ARPGSamurai_Attack_Combo3_Montage" :`3` "/Game/Character/SamuraiAnimation/RootMotion/Anim_ARPGSamurai_Attack_Combo4_Montage.Anim_ARPGSamurai_Attack_Combo4_Montage" :!type "AnimMontage Object Reference")))
  (return _returnvalue))

(fn `UserConstructionScript`
  (`SceneComponent.K2_AttachToComponent` (`self.WeaponMesh`) (`self.Mesh`) "Weapon" "KeepRelative" "KeepRelative" "KeepRelative" true)
  (`HitTraceComponent.InitWeapon` (`self. Hit Box Trace`) (`self.WeaponMesh`)))