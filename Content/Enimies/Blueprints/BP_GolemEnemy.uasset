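; Golem enemy character that rises with a montage on spawn, sets up its state info and weapon line trace, and binds front and back health bar widgets.
; AI perception and the absolute and memory range volumes report the player's sight and proximity changes to EnemyMemory.
; Animation hooks play a hit reaction or one of three stage-selected attacks, including an AoE.
; Falling down stops the montage and calls Drop.
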(event `self.ReceiveBeginPlay`
  (`self.SetUpStateInfo`)
  (`HitTraceComponent.InitWeapon` (`self.Hit Line Trace`) (`self.Mesh`))
  (bind _asenemy_health_bar (cast `EnemyHealthBar` (`WidgetComponent.GetUserWidgetObject` (`self.Health Bar`))))
  (`EnemyHealthBar.InitEnemy` _asenemy_health_bar self)
  (bind _asenemy_health_bar_2 (cast `EnemyHealthBar` (`WidgetComponent.GetUserWidgetObject` (`self.Heath Bar Back`))))
  (`EnemyHealthBar.InitEnemy` _asenemy_health_bar_2 self)
  (`self.PlayAnimMontage` "/Game/Enimies/Golem/Animations/Anim_Rise_Montage.Anim_Rise_Montage"))

(event `self.EnemyFallDown`
  (`self.StopAnimMontage` null)
  (`self.Drop`))

(event `self.AIPerception.OnTargetPerceptionUpdated`
  (params (Actor :type "Actor Object Reference") (Stimulus :type "AIStimulus Structure"))
  (bind _enemymemory (`self.EnemyMemory`))
  (cast `PlayerCharacterCPP` Actor)
  (if (`.bSuccessfullySensed` (break `AIStimulus` Stimulus))
    (`EnemyMemory.PlayerEnterSight` _enemymemory)
    (else
      (`EnemyMemory.PlayerOutSight` _enemymemory))))

(event `self.Absolute Range.OnComponentBeginOverlap`
  (params (OverlappedComponent :type "PrimitiveComponent Object Reference") (OtherActor :type "Actor Object Reference") (OtherComp :type "PrimitiveComponent Object Reference") (OtherBodyIndex :type Integer) (bFromSweep :type Boolean) (SweepResult :type "HitResult Structure (by ref)"))
  (cast `PlayerCharacterCPP` OtherActor)
  (`EnemyMemory.PlayerEnterAbsoluteRange` (`self.EnemyMemory`)))

(event `self.Absolute Range.OnComponentEndOverlap`
  (params (OverlappedComponent :type "PrimitiveComponent Object Reference") (OtherActor :type "Actor Object Reference") (OtherComp :type "PrimitiveComponent Object Reference") (OtherBodyIndex :type Integer))
  (cast `PlayerCharacterCPP` OtherActor)
  (`EnemyMemory.PlayerOutAbsoluteRange` (`self.EnemyMemory`)))

(event `self.Memory Range.OnComponentBeginOverlap`
  (params (OverlappedComponent :type "PrimitiveComponent Object Reference") (OtherActor :type "Actor Object Reference") (OtherComp :type "PrimitiveComponent Object Reference") (OtherBodyIndex :type Integer) (bFromSweep :type Boolean) (SweepResult :type "HitResult Structure (by ref)"))
  (cast `PlayerCharacterCPP` OtherActor)
  (`EnemyMemory.PlayerEnterMemoryRange` (`self.EnemyMemory`)))

(event `self.Memory Range.OnComponentEndOverlap`
  (params (OverlappedComponent :type "PrimitiveComponent Object Reference") (OtherActor :type "Actor Object Reference") (OtherComp :type "PrimitiveComponent Object Reference") (OtherBodyIndex :type Integer))
  (cast `PlayerCharacterCPP` OtherActor)
  (`EnemyMemory.PlayerOutMemoryRange` (`self.EnemyMemory`)))

(event `self.PlayHittedAnime`
  (`self.PlayAnimMontage` "/Game/Enimies/Golem/Animations/Anim_Hit_Montage.Anim_Hit_Montage"))

(fn `PlayAttackAnime`
  (params (Stage :type Integer))
  (returns (ReturnValue :type "Float (double-precision)"))
  (bind _returnvalue (`self.PlayAnimMontage` (select `int` Stage :`0` "/Game/Enimies/Golem/Animations/Anim_Attack1_Montage.Anim_Attack1_Montage" :`1` "/Game/Enimies/Golem/Animations/Anim_Attack2_Montage.Anim_Attack2_Montage" :`2` "/Game/Enimies/Golem/Animations/Anim_Attack_AoE_Montage.Anim_Attack_AoE_Montage" :!type "AnimMontage Object Reference")))
  (return _returnvalue))

(fn `UserConstructionScript`)