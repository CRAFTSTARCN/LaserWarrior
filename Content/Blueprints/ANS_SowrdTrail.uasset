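; Anim notify state that toggles a Niagara effect on the animated actor, named for a sword trail.
; On begin, it finds the mesh owner's Niagara component by class and activates it with a reset.
; On end, it deactivates that component.
; The lookup takes whichever Niagara component the class search returns, so it does not target a specific trail by name or tag.
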(fn `Received_NotifyBegin`
  (params (MeshComp :type "SkeletalMeshComponent Object Reference") (Animation :type "AnimSequenceBase Object Reference") (TotalDuration :type "Float (double-precision)"))
  (returns (ReturnValue :type Boolean))
  (bind _returnvalue (`Actor.GetComponentByClass` (`ActorComponent.GetOwner` MeshComp) "/Script/Niagara.NiagaraComponent"))
  (`/Engine/EditorBlueprintResources/StandardMacros.IsValid` _returnvalue
    (:`Is Valid`
      (`ActorComponent.Activate` _returnvalue true)
      (return true))
    (:`Is Not Valid`
      (return false))))

(fn `Received_NotifyEnd`
  (params (MeshComp :type "SkeletalMeshComponent Object Reference") (Animation :type "AnimSequenceBase Object Reference"))
  (returns (ReturnValue :type Boolean))
  (bind _returnvalue (`Actor.GetComponentByClass` (`ActorComponent.GetOwner` MeshComp) "/Script/Niagara.NiagaraComponent"))
  (`/Engine/EditorBlueprintResources/StandardMacros.IsValid` _returnvalue
    (:`Is Valid`
      (`ActorComponent.Deactivate` _returnvalue)
      (return false))
    (:`Is Not Valid`
      (return false))))