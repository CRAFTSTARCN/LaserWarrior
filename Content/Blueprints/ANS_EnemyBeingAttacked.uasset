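; Anim notify state that marks an Enemy as being hit for the duration of its window in an animation.
; On begin it casts the mesh owner to Enemy and sets IsBeingHitted to true, then clears it on end.
; Both callbacks return false when the owner is not an Enemy.
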(fn `Received_NotifyBegin`
  (params (MeshComp :type "SkeletalMeshComponent Object Reference") (Animation :type "AnimSequenceBase Object Reference") (TotalDuration :type "Float (double-precision)"))
  (returns (ReturnValue :type Boolean))
  (bind _asenemy (cast `Enemy` (`ActorComponent.GetOwner` MeshComp))
    (:`then`
      (set `Enemy.bIsBeingHitted` true _asenemy)
      (return true))
    (:`CastFailed`
      (return false))))

(fn `Received_NotifyEnd`
  (params (MeshComp :type "SkeletalMeshComponent Object Reference") (Animation :type "AnimSequenceBase Object Reference"))
  (returns (ReturnValue :type Boolean))
  (bind _asenemy (cast `Enemy` (`ActorComponent.GetOwner` MeshComp))
    (:`then`
      (set `Enemy.bIsBeingHitted` false _asenemy)
      (return true))
    (:`CastFailed`
      (return false))))