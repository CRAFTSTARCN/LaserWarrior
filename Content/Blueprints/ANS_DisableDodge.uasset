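; Anim notify state that blocks the player's dodge for the span it covers in an animation.
; On begin it casts player controller 0 to ARPGPlayerController and clears AllowDodge, and on end it sets the flag back to true.
; It always targets the first player's controller rather than the mesh owner, and restores the flag without saving its previous value.
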(fn `Received_NotifyBegin`
  (params (MeshComp :type "SkeletalMeshComponent Object Reference") (Animation :type "AnimSequenceBase Object Reference") (TotalDuration :type "Float (double-precision)"))
  (returns (ReturnValue :type Boolean))
  (bind _asarpgplayer_controller (cast `ARPGPlayerController` (`GameplayStatics.GetPlayerController` MeshComp))
    (:`then`
      (set `ARPGPlayerController.bAllowDodge` false _asarpgplayer_controller)
      (return true))
    (:`CastFailed`
      (return false))))

(fn `Received_NotifyEnd`
  (params (MeshComp :type "SkeletalMeshComponent Object Reference") (Animation :type "AnimSequenceBase Object Reference"))
  (returns (ReturnValue :type Boolean))
  (bind _asarpgplayer_controller (cast `ARPGPlayerController` (`GameplayStatics.GetPlayerController` MeshComp))
    (:`then`
      (set `ARPGPlayerController.bAllowDodge` true _asarpgplayer_controller)
      (return true))
    (:`CastFailed`
      (return false))))